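; Grid tactics ability that lets the player move the owning unit or attack another, spending action points.
; Activation branches on remaining AP to show pathfound move tiles, only targets, or switch to Idle.
; Hover draws spline paths; left clicks pay AP, then ExecuteAbility moves the unit or queues an Attack action.
; The Play state gates activation and the queued Attack, which delegates to the attacking BP_CharacterUnit.
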(event EventBeginPlay
  (|CallParentFunction) ; This node is disabled and will not be called.\nDrag off pins to build functionality.
)

(event EventServerHover
  (params (bValidTile :type Boolean) (GridIndex :type Integer) (Location :type Vector :default "0, 0, 0"))
  (bind _gridmanagerref (Variables|Default|GetGridManagerRef))
  (bind _hoveredtile (Variables|Default|GetHoveredTile))
  (bind _gridunits (Variables|/Game/AdvancedTurnBasedTileToolkit/Core/Grid/BP_GridManager.BP_GridManager_C|GetGridUnits _gridmanagerref))
  (bind (_value _returnvalue) (Utilities|Map|Find _gridunits _hoveredtile))
  ;[1 1 1] Hover over tiles, spline pathing.  Does not have functionality, it just shows the spline path and where the mouse is hovered over
  (CallFunction|CallClientHoverfromServer bValidTile GridIndex)
  (CallFunction|ClientClearPath)
  (if bValidTile
    (if (not (Default|CheckifImpassable (Variables|Default|GetGridManagerRef) (Variables|Default|GetHoveredTile))) ; Never show path if tile is impassable
      (if _returnvalue
        (if (and (== _value (Variables|Default|GetOwningUnit)) (!= (Variables|/Game/AdvancedTurnBasedTileToolkit/Core/Grid/BP_GridActor.BP_GridActor_C|GetGridIndex (Variables|Default|GetOwningUnit)) (Variables|Default|GetHoveredTile))) ; To allow for big units to move onto tiles it is occupying
          (if (Utilities|Map|Contains (Variables|Default|GetStoredPathsMap) (Variables|Default|GetHoveredTile)) :!label _label ; Only show path if the current tile has a move cost (e.g. is reachable)
            (bind _pathlocations (Default|FindSplinePathtoGridIndex (Variables|Default|GetGridManagerRef) (Variables|Default|GetStoredPathsMap) (Variables|Default|GetHoveredTile) (Variables|/Game/AdvancedTurnBasedTileToolkit/Core/Grid/BP_GridActor.BP_GridActor_C|GetAnchorOffset (Variables|Default|GetOwningUnit)) 0 "Linear"))
            (CallFunction|ClientDisplayPath _pathlocations (Variables|Default|GetSplineType))))
        (else
          (goto _label))))))

(event EventServerInteract
  (params (bValidTile :type Boolean) (Index :type Integer) (Location :type Vector :default "0, 0, 0") (Key :type Key%20Structure :default "None") (bReleased :type Boolean) (ClickType :type EClickType%20Enum :default "NewEnumerator0") (CallingPc :type BP%20Player%20Controller%20ATBTT%20Object%20Reference))
  (bind _owningunit (Variables|Default|GetOwningUnit))
  (bind _clickedindex (Variables|Default|GetClickedIndex))
  (bind _clickedindex_2 (Variables|Default|GetClickedIndex))
  (bind _storedpathsmap (Variables|Default|GetStoredPathsMap))
  (bind _owningunit_2 (Variables|Default|GetOwningUnit))
  (bind _storedpathsmap_2 (Variables|Default|GetStoredPathsMap))
  (bind _clickedindex_3 (Variables|Default|GetClickedIndex))
  (bind _gridmanagerref (Variables|Default|GetGridManagerRef))
  (bind _value (Utilities|Map|Find _storedpathsmap _clickedindex_3))
  (bind _value_2 (Utilities|Map|Find _storedpathsmap_2 _clickedindex))
  (bind _gridunits (Variables|/Game/AdvancedTurnBasedTileToolkit/Core/Grid/BP_GridManager.BP_GridManager_C|GetGridUnits _gridmanagerref))
  (bind (_value_3 _returnvalue) (Utilities|Map|Find _gridunits _clickedindex_2))
  ;[1 1 1] Events Based on clicking left mouse button and right mouse button
  ;;[0.272 0.3646 0.09923] Left click, valid tile
  (switch Utilities|FlowControl|Switch|SwitchonEClickType ClickType
    (:NewEnumerator0
      (if bValidTile
        ;;[0.7188 0.7063 0.09729] Left click released, suggested hover true, execute
        (if bReleased
          (if (Variables|Default|GetbSuggestHover)
            (CallFunction|ExecuteSuggested)
            (elif (Utilities|Set|Contains (Variables|Default|GetPossibleTargets) (Variables|Default|GetClickedIndex))
              ;;[1 0 0] Enemy in way, queue attack
              (CallFunction|PayAPCost false)
              (Utilities|SimpleQueue self "Clear" "NewEnumerator0" true :!label _label)
              (CallFunction|ExecuteAbility (Variables|Default|GetClickedIndex))
              (CallFunction|Deactivate)
              (if (Utilities|IsValid (Variables|Default|GetOwningUnit))
                (CallFunction|SignalAbilityExecuted))
              (else
                ;;[1 0.09705 0.8588] No enemies found, can move if within range
                (if (Math|Boolean|ANDBoolean (>= (Variables|Default|GetPossibleMove) (.cost _value_2)) (> (.cost _value_2) 0) (or (not _returnvalue) (Math|Boolean|ANDBoolean _returnvalue (== _value_3 _owningunit_2) (!= (Variables|/Game/AdvancedTurnBasedTileToolkit/Core/Grid/BP_GridActor.BP_GridActor_C|GetGridIndex _owningunit_2) (Variables|Default|GetClickedIndex)))))
                  ;;[0.6198 0.04898 0.4902] Check to see if the move is in range
                  (if (and (>= (Variables|Default|GetPossibleMove) (.cost _value)) (> (.cost _value) 0))
                    (CallFunction|PayMoveAPCost (Variables|Default|GetClickedIndex) (Variables|Default|GetStoredPathsMap) (Variables|Default|GetMoveCostType))
                    (goto _label))
                  (elif _returnvalue
                    (if (== (.Value (Utilities|Map|Find (Variables|/Game/AdvancedTurnBasedTileToolkit/Core/Grid/BP_GridManager.BP_GridManager_C|GetGridUnits (Variables|Default|GetGridManagerRef)) (Variables|Default|GetClickedIndex))) (Variables|Default|GetOwningUnit))
                      (Variables|/Game/AdvancedTurnBasedTileToolkit/Core/Units/BP_Unit.BP_Unit_C|SetCurrentAP _owningunit (Math|Integer|Max(Integer) (- (Variables|/Game/AdvancedTurnBasedTileToolkit/Core/Units/BP_Unit.BP_Unit_C|GetCurrentAP _owningunit) 1)))
                      (CallFunction|SignalAbilityExecuted)
                      (else
                        (CallFunction|DefaultClick (Variables|Default|GetClickedIndex) Location)))
                    (elif (< (Variables|/Game/AdvancedTurnBasedTileToolkit/Core/Units/BP_Unit.BP_Unit_C|GetCurrentAP (Variables|Default|GetOwningUnit)) 2)
                      (Variables|/Game/AdvancedTurnBasedTileToolkit/Core/Units/BP_Unit.BP_Unit_C|SetCurrentAP (Variables|Default|GetOwningUnit) 0)
                      (CallFunction|SignalAbilityExecuted))))))))))))

(event EventTick
  (params (DeltaSeconds :type Float%20%28single-precision%29)))

(event EventPlayerActivate
  (params (Unit :type BP%20Unit%20Object%20Reference))
  (bind _returnvalue (Game|GetPlayerController 0))
  (bind _play (Variables|Default|Getplay))
  (bind _owningunit (Variables|Default|GetOwningUnit))
  (bind _owningunit_2 (Variables|Default|GetOwningUnit))
  (bind _size (Variables|/Game/AdvancedTurnBasedTileToolkit/Core/Units/BP_Unit.BP_Unit_C|GetSize _owningunit_2))
  ;[1 1 1] Comment
  (if (or (Utilities|Enum|Equal(Enum) _play "NewEnumerator0") (Utilities|Enum|Equal(Enum) _play "NewEnumerator1"))
    (switch int (Variables|/Game/AdvancedTurnBasedTileToolkit/Core/Units/BP_Unit.BP_Unit_C|GetCurrentAP Unit)
      (:Default
        ;;[1 1 1] Blue tiles from both
        (Utilities|FlowControl|Sequence
          (:then_0
            (bind _pathsmap (Default|RunPathfinding (Variables|Default|GetGridManagerRef) (Variables|/Game/AdvancedTurnBasedTileToolkit/Core/Grid/BP_GridActor.BP_GridActor_C|GetGridIndex _owningunit) (Variables|Default|GetPossibleMove) (Variables|/Game/AdvancedTurnBasedTileToolkit/Core/Units/BP_Unit.BP_Unit_C|GetPathfindingType _owningunit) false))
            (Variables|Default|SetStoredPathsMap _pathsmap)
            (Utilities|Array|Clear (Variables|Default|GetStoredLocations))
            (bind _keys (Utilities|Map|Keys (Variables|Default|GetStoredPathsMap)))
            (if (> _size 1)
              (bind _biggridindexes (Default|FindBigIndexesfromIndexes (Variables|Default|GetGridManagerRef) _keys _size))
              (Variables|Default|SetMoveDisplayIndexes _biggridindexes)
              (else
                (Variables|Default|SetMoveDisplayIndexes _keys)))
            (for _array_element (Variables|Default|GetMoveDisplayIndexes)
              (if (not (Utilities|Map|Contains (Variables|/Game/AdvancedTurnBasedTileToolkit/Core/Grid/BP_GridManager.BP_GridManager_C|GetGridUnits (Variables|Default|GetGridManagerRef)) _array_element))
                (Utilities|Array|Add (Variables|Default|GetStoredLocations) (.Value (Utilities|Map|Find (Variables|/Game/AdvancedTurnBasedTileToolkit/Core/Grid/BP_GridManager.BP_GridManager_C|GetGridLocations (Variables|Default|GetGridManagerRef)) _array_element)))))
            (Utilities|QueueAction self "DisplayMoveTiles" "NewEnumerator1" true -1 false 0.0 0 0 0 0 (Variables|Default|GetStoredLocations)))
          (:then_1
            (Variables|Default|SetbDisplayInvalidTiles false)
            (|CallParentFunction (Variables|Default|GetOwningUnit)))))
      (:0
        (Class|BPIAbility|ActivateAbility(Message) _returnvalue "/Game/AdvancedTurnBasedTileToolkit/Core/Abilities/BP_AbilityBase_Idle.BP_AbilityBase_Idle_C" _returnvalue) ; TODO: check for multiplayer
      )
      (:1
        (Variables|Default|SetbDisplayInvalidTiles false)
        (Utilities|Map|Clear (Variables|Default|GetStoredPathsMap))
        (|CallParentFunction (Variables|Default|GetOwningUnit))))))

(event EventAttack
  (params (Attacker :type BP%20Unit%20Object%20Reference) (TargetUnit :type BP%20Unit%20Object%20Reference) (Damage :type Float%20%28single-precision%29))
  ;[1 1 1] Executing object is reference, array of units is copy
  (if (Utilities|Enum|Equal(Enum) (Variables|Default|Getplay) "NewEnumerator1")
    ;;[1 1 1] attacker
    (bind _asbp_character_unit (Utilities|Casting|CastToBP_CharacterUnit Attacker))
    ;;[1 1 1] victim
    (bind _asbp_character_unit_2 (Utilities|Casting|CastToBP_CharacterUnit TargetUnit))
    (Default|Attack _asbp_character_unit _asbp_character_unit_2)
    (else
      (Development|PrintString "Can't attack, tried to tho")
      (CallFunction|PlayerActivate Attacker)))
  (Utilities|EndAction))

(event Collision|EventActorBeginOverlap
  (params (OtherActor :type Actor%20Object%20Reference)))

(event EventActivate
  (params (bReassess :type Boolean) (OwningActor :type Actor%20Object%20Reference))
  (|CallParentFunction bReassess OwningActor))

(fn ConstructionScript
  (|CallParentFunction))

(fn ExecuteAbility
  (params (TargetIndex :type Integer))
  (bind _gridmanagerref (Variables|Default|GetGridManagerRef))
  (bind _gridunits (Variables|/Game/AdvancedTurnBasedTileToolkit/Core/Grid/BP_GridManager.BP_GridManager_C|GetGridUnits _gridmanagerref))
  (bind (_value _returnvalue) (Utilities|Map|Find _gridunits TargetIndex))
  (if _returnvalue
    (if (!= _value (Variables|Default|GetOwningUnit))
      (Utilities|QueueAction self "Attack" "NewEnumerator0" false -1 false 0.0 0 0 (Utilities|Array|MakeArray (Variables|Default|GetDamage)) 0 0 0 0 (Utilities|Array|MakeArray (Variables|Default|GetOwningUnit) (.Value (Utilities|Map|Find (Variables|/Game/AdvancedTurnBasedTileToolkit/Core/Grid/BP_GridManager.BP_GridManager_C|GetGridUnits (Variables|Default|GetGridManagerRef)) TargetIndex))))
      (Utilities|SimpleQueue self "HideTargetMarker" "NewEnumerator0" true)
      (return true)
      (else
        _)))
  (Default|ShowUnitSelect (Variables|Default|GetOwningUnit))
  (Default|MovetoIndex (Variables|Default|GetOwningUnit) TargetIndex (Variables|Default|GetStoredPathsMap))
  (CallFunction|ClientShowTargetMarker (.Value (Utilities|Map|Find (Variables|/Game/AdvancedTurnBasedTileToolkit/Core/Grid/BP_GridManager.BP_GridManager_C|GetGridLocations (Variables|Default|GetGridManagerRef)) TargetIndex)) true)
  (Utilities|SimpleQueue self "HideTargetMarker" "NewEnumerator0" true)
  (return false))

(fn ChangePlay
  (params (NewPlay :type PlaySelectionState%20Enum :default "NewEnumerator3"))
  (bind _output_get (Variables|Default|Setplay NewPlay))
  (Development|PrintString (Utilities|String|EnumtoString _output_get)))

(fn RunMove
  (params (Unit :type BP%20Unit%20Object%20Reference))
  (CallFunction|PlayerActivate Unit))

(fn SignalAbilityExecuted
  (|CallParentFunction))